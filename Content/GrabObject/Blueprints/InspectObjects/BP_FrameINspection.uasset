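; Inspectable object Blueprint, named as a frame, that reveals a key when the player rotates it to the correct orientation.
; It extends parent inspection events, creating a WB_InspectObject info widget at BeginPlay with the key's image and name.
; Rotation checks toggle a prompt component and the info widget during the first step.
; Interacting while in position hides the item mesh and both widgets, then advances the step index.
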(event `self.ReceiveBeginPlay`
  ;[1 1 1] Information about the item
  (`parent.ReceiveBeginPlay`)
  (bind _returnvalue (`|CreateWidget` "/ObjectInspection/GrabObject/GUI/WB_InspectObject.WB_InspectObject_C"))
  (bind _output_get (set `self.InfoWidget` _returnvalue))
  (set `InspectionObjectInfWidget.ItemImage` "/ObjectInspection/GrabObject/Textures/T_Key.T_Key" _output_get)
  (set `InspectionObjectInfWidget.ItemName` "Key" _output_get))

(event `self.RemoveWidgets`
  (bind _infowidget (`self.InfoWidget`))
  ;[1 1 1] Remove Widgets on Interact End
  (`parent.RemoveWidgets`)
  (if (`Widget.IsInViewport` _infowidget)
    (`Widget.RemoveFromParent` _infowidget)))

(event `self.InteractToActor`
  ;[1 1 1] If you are in position - do some event
  (`parent.InteractToActor`)
  (if (`self.onPosition`)
    (switch `int` (`self.stepIndex`)
      (:`0`
        (`SceneComponent.SetHiddenInGame` (`self.ItemMeshComp`) true false)
        (`SceneComponent.SetHiddenInGame` (`self.Widget1`) true false)
        (`Widget.RemoveFromParent` (`self.InfoWidget`))
        (`/Engine/EditorBlueprintResources/StandardMacros.IncrementInt` (`self.stepIndex`))))))

(event `self.TestRotation`
  (bind _infowidget (`self.InfoWidget`))
  ;[1 1 1] Check is you are on the current rotation every move tick
  (`parent.TestRotation`)
  (bind _returnvalue (`self.OnCurrentDirection`))
  (bind _output_get (set `self.onPosition` _returnvalue))
  (if _output_get
    (switch `int` (`self.stepIndex`)
      (:`0`
        (`SceneComponent.SetVisibility` (`self.Widget1`) true false)
        (if (not (`Widget.IsInViewport` _infowidget))
          (`UserWidget.AddToViewport` _infowidget 0))))
    (else
      (switch `int` (`self.stepIndex`)
        (:`0`
          (`SceneComponent.SetVisibility` (`self.Widget1`) false false)
          (`Widget.RemoveFromParent` (`self.InfoWidget`)))))))

(fn `UserConstructionScript`)